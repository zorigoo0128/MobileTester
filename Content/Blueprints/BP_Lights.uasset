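; BP_Lights is a lighting controller actor that switches a level between day and night looks through a Day boolean.
; Its Construction Script rotates the referenced DirectionalLight, sets SkyLight intensity and color (white for day, blue for night), and toggles SkySphere cloud opacity before refreshing its material.
; The switch applies at construction only, with no active BeginPlay or Tick logic.
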(event EventBeginPlay)

(event EventTick
  (params (DeltaSeconds :type Float%20%28single-precision%29)))

(fn ConstructionScript
  (bind _skysphere (Variables|Default|GetSkySphere))
  (bind _directionallight (Variables|Default|GetDirectionalLight))
  (bind _skylight (Variables|Default|GetSkyLight))
  (bind _skylight_2 (Variables|Default|GetSkyLight))
  (bind _lightcomponent (Variables|/Script/Engine.SkyLight|GetLightComponent _skylight))
  (bind _lightcomponent_2 (Variables|/Script/Engine.SkyLight|GetLightComponent _skylight_2))
  (if (Variables|Default|GetDay?)
    (Transformation|SetActorRotation _directionallight "-45.000000, 0, 0")
    (Rendering|Components|Light|SetIntensity _lightcomponent 1.0)
    (Rendering|Components|Light|SetLightColor _lightcomponent_2 "(R=1.000000,G=1.000000,B=1.000000,A=1.000000)")
    (Variables|/Engine/EngineSky/BP_Sky_Sphere.BP_Sky_Sphere_C|SetCloud%20opacity _skysphere 1.0)
    (Default|RefreshMaterial _skysphere)
    (else
      (Transformation|SetActorRotation _directionallight "70.000000, 0, 0")
      (Rendering|Components|Light|SetIntensity _lightcomponent 1e+01)
      (Rendering|Components|Light|SetLightColor _lightcomponent_2 "(R=0.000000,G=0.175449,B=0.291667,A=1.000000)")
      (Variables|/Engine/EngineSky/BP_Sky_Sphere.BP_Sky_Sphere_C|SetCloud%20opacity _skysphere 0.0)
      (Default|RefreshMaterial _skysphere))))